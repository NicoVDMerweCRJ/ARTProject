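; BP_Intro_Elephant is an intro elephant actor that animates and trumpets on a timed script.
; On BeginPlay, its elephant mesh loops a walk animation, then switches to a looping idle after one second.
; In parallel, a delayed 2D trumpet sound plays five seconds in.
; Disconnected timeline chains for fading the material Opacity parameter out and in are present but never run.
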(event `self.ReceiveBeginPlay`
  (`|ExecutionSequence`
    (:`then_0`
      (`SkeletalMeshComponent.PlayAnimation` (`self.SM_Elephant_Idle`) "/Game/Creative/Assets/3D_Assets/Elephant/Animations/Anim_Elephant_Walk.Anim_Elephant_Walk" true)
      (`KismetSystemLibrary.Delay` 1.0)
      (`SkeletalMeshComponent.PlayAnimation` (`self.SM_Elephant_Idle`) "/Game/Creative/Assets/3D_Assets/Elephant/Animations/Anim_Elephant_Idle.Anim_Elephant_Idle" true))
    (:`then_1`
      (`KismetSystemLibrary.Delay` 5.0)
      (`GameplayStatics.PlaySound2D` "/Game/Creative/Assets/Audio/527845__d-jones__elephant-trumpets-growls.527845__d-jones__elephant-trumpets-growls" 1.0 1.0 0.0 null null))))

(fn `UserConstructionScript`)