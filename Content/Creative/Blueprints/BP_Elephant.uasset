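; BP_Elephant is a scripted elephant character that introduces itself with animation, sound and text when spawned.
; On BeginPlay a puff particle hides its appearance, then the skeletal mesh is revealed and the puff is destroyed.
; A Sequence then runs two Delay-timed tracks: one alternates idle, walk and run animations.
; The other plays trumpet sounds and toggles a text bubble, changing it to "I'm Oli!" for the second showing.
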(event `self.ReceiveBeginPlay`
  (bind _textrender (`self.TextRender`))
  (bind _textrender_2 (`self.TextRender`))
  (`ActorComponent.SetActive` (`self.P_Puff1`) true false)
  (`KismetSystemLibrary.Delay` 0.1)
  (`SceneComponent.SetVisibility` (`self.SM_Elephant_Idle`) true false)
  (`KismetSystemLibrary.Delay` 0.7)
  (`ActorComponent.K2_DestroyComponent` (`self.P_Puff1`))
  (`|ExecutionSequence`
    (:`then_0`
      (`SkeletalMeshComponent.PlayAnimation` (`self.SM_Elephant_Idle`) "/Game/Creative/Assets/3D_Assets/Elephant/Animations/Anim_Elephant_Idle.Anim_Elephant_Idle" true)
      (`KismetSystemLibrary.Delay` 0.5)
      (`SkeletalMeshComponent.PlayAnimation` (`self.SM_Elephant_Idle`) "/Game/Creative/Assets/3D_Assets/Elephant/Animations/Anim_Elephant_Walk.Anim_Elephant_Walk" false)
      (`KismetSystemLibrary.Delay` 1.0)
      (`SkeletalMeshComponent.PlayAnimation` (`self.SM_Elephant_Idle`) "/Game/Creative/Assets/3D_Assets/Elephant/Animations/Anim_Elephant_Idle.Anim_Elephant_Idle" true)
      (`KismetSystemLibrary.Delay` 1.5)
      (`SkeletalMeshComponent.PlayAnimation` (`self.SM_Elephant_Idle`) "/Game/Creative/Assets/3D_Assets/Elephant/Animations/Anim_Elephant_Run.Anim_Elephant_Run" false)
      (`KismetSystemLibrary.Delay` 1.0)
      (`SkeletalMeshComponent.PlayAnimation` (`self.SM_Elephant_Idle`) "/Game/Creative/Assets/3D_Assets/Elephant/Animations/Anim_Elephant_Idle.Anim_Elephant_Idle" true))
    (:`then_1`
      (`KismetSystemLibrary.Delay` 0.5)
      (`GameplayStatics.PlaySound2D` "/Game/Creative/Assets/Audio/527845__d-jones__elephant-trumpets-growls.527845__d-jones__elephant-trumpets-growls" 0.5 1.0 0.0 null null)
      (`SceneComponent.SetVisibility` _textrender_2 true false)
      (`SceneComponent.SetVisibility` (`self.Text_Plane_Front`) true false)
      (`SceneComponent.SetVisibility` (`self.Text_Plane_Back`) true false)
      (`KismetSystemLibrary.Delay` 2.5)
      (`SceneComponent.SetVisibility` _textrender_2 false false)
      (`SceneComponent.SetVisibility` (`self.Text_Plane_Front`) false false)
      (`SceneComponent.SetVisibility` (`self.Text_Plane_Back`) false false)
      (`KismetSystemLibrary.Delay` 1.0)
      (bind _output_get (set `self.TestString` "I'm Oli!"))
      (`TextRenderComponent.K2_SetText` _textrender _output_get)
      (`GameplayStatics.PlaySound2D` "/Game/Creative/Assets/Audio/527845__d-jones__elephant-trumpets-growls.527845__d-jones__elephant-trumpets-growls" 0.5 1.0 0.0 null null)
      (`SceneComponent.SetVisibility` _textrender true false)
      (`SceneComponent.SetVisibility` (`self.Text_Plane_Front`) true false)
      (`SceneComponent.SetVisibility` (`self.Text_Plane_Back`) true false)
      (`KismetSystemLibrary.Delay` 3.0)
      (`SceneComponent.SetVisibility` _textrender false false)
      (`SceneComponent.SetVisibility` (`self.Text_Plane_Front`) false false)
      (`SceneComponent.SetVisibility` (`self.Text_Plane_Back`) false false))))

(fn `UserConstructionScript`)