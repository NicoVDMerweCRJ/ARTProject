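; BP_Intro_Main is an intro sequence actor that stages a timed elephant reveal, then cleans itself up.
; A chain of delays from BeginPlay shows the elephant, then destroys the puff cloud component shortly after.
; It later adds a child actor component at a fixed sideways offset and, after a longer wait, destroys the whole actor.
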(event `self.ReceiveBeginPlay`
  (`KismetSystemLibrary.Delay` 0.2)
  (`SceneComponent.SetVisibility` (`self.BP_Intro_Elephant`) true false)
  (`KismetSystemLibrary.Delay` 0.7)
  (`ActorComponent.K2_DestroyComponent` (`self.PS_2D_Puff_Cloud_Big`))
  (`KismetSystemLibrary.Delay` 3.0)
  (bind _output_get (set `self.Par_Spawn_Location` (0.0 213.0 0.0)))
  (`AddComponent|NODE_AddChildActorComponent-0` :`RelativeTransform` (`KismetMathLibrary.Conv_VectorToTransform` _output_get))
  (`KismetSystemLibrary.Delay` 10.0)
  (`self.K2_DestroyActor`))

(fn `UserConstructionScript`)