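; BP_Intro_Text is an intro title actor that animates mesh letters (O, L, I base and I top) with sound.
; On BeginPlay, timelines move the I parts and L vertically while material Opacity parameters fade the letters in, some after short delays.
; Applause plays immediately, followed by a tada sound.
; A delayed final timeline fades out all letters and a sphere.
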(event `self.ReceiveBeginPlay`
  (bind _text_sm_i_top (`self.Text_SM_I_Top`))
  (`|ExecutionSequence`
    (:`then_0`
      (`KismetSystemLibrary.Delay` 1.5)
      (bind (_direction _fade_in) (`Timeline|Timeline_0`)
        (:`Update`
          (`|ExecutionSequence`
            (:`then_0`
              (`MeshComponent.SetScalarParameterValueOnMaterials` (`self.Text_SM_O`) "Opacity" _fade_in))
            (:`then_1`
              (`MeshComponent.SetScalarParameterValueOnMaterials` (`self.Text_SM_L`) "Opacity" _fade_in))
            (:`then_2`
              (`MeshComponent.SetScalarParameterValueOnMaterials` (`self.Text_SM_I_Base`) "Opacity" _fade_in))))))
    (:`then_1`
      (bind (_direction_2 _move_down _move_up) (`Timeline|Move_Down_Object`)
        (:`Update`
          (`|ExecutionSequence`
            (:`then_0`
              (`SceneComponent.K2_SetWorldLocation` (`self.Text_SM_I_Base`) (`KismetMathLibrary.MakeVector` 0.0 0.0 _move_down) false false))
            (:`then_1`
              (`SceneComponent.K2_SetWorldLocation` (`self.Text_SM_L`) (`KismetMathLibrary.MakeVector` 0.0 0.0 _move_up) false false))))))
    (:`then_2`
      (`KismetSystemLibrary.Delay` 0.1)
      (bind (_direction_3 _move_down_2 _fade_in_2) (`Timeline|I_Top_Func`)
        (:`Update`
          (`|ExecutionSequence`
            (:`then_0`
              (`SceneComponent.K2_SetWorldLocation` _text_sm_i_top (`KismetMathLibrary.MakeVector` 0.0 0.0 _move_down_2) false false))
            (:`then_1`
              (`MeshComponent.SetScalarParameterValueOnMaterials` _text_sm_i_top "Opacity" _fade_in_2))))))
    (:`then_3`
      (`GameplayStatics.PlaySound2D` "/Game/Creative/Assets/Audio/74439__robinhood76__01080-children-applause-34.74439__robinhood76__01080-children-applause-34" 0.2 1.0 0.0 null null)
      (`KismetSystemLibrary.Delay` 2.0)
      (`GameplayStatics.PlaySound2D` "/Game/Creative/Assets/Audio/376318__jimhancock__tada.376318__jimhancock__tada" 1.0 1.0 0.0 null null))
    (:`then_4`
      (`KismetSystemLibrary.Delay` 8.0)
      (bind (_direction_4 _fade_in_3 _fade_out) (`Timeline|Timeline_1`)
        (:`Update`
          (`|ExecutionSequence`
            (:`then_0`
              (`MeshComponent.SetScalarParameterValueOnMaterials` (`self.Sphere`) "Opacity" _fade_out))
            (:`then_1`
              (`MeshComponent.SetScalarParameterValueOnMaterials` (`self.Text_SM_O`) "Opacity" _fade_out))
            (:`then_2`
              (`MeshComponent.SetScalarParameterValueOnMaterials` (`self.Text_SM_L`) "Opacity" _fade_out))
            (:`then_3`
              (`MeshComponent.SetScalarParameterValueOnMaterials` (`self.Text_SM_I_Base`) "Opacity" _fade_out))
            (:`then_4`
              (`MeshComponent.SetScalarParameterValueOnMaterials` (`self.Text_SM_I_Top`) "Opacity" _fade_out))))))))

(fn `UserConstructionScript`)